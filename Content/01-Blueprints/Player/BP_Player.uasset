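; BP_Player is the pirate player character, handling movement, respawning and coin collection.
; BeginPlay adds the Enhanced Input mapping context, stores the starting transform and creates the HUD, all behind a subsystem validity check.
; Input drives camera-yaw-relative movement, look and jump.
; PlayerDeath teleports the player to the respawn transform, which Checkpoint overwrites, while AddCoin updates the running total and pushes it to the HUD.
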(event `self.ReceiveBeginPlay`
  (bind _returnvalue (pcsubsystem `EnhancedInputLocalPlayerSubsystem` (`GameplayStatics.GetPlayerController` 0)))
  (`/Engine/EditorBlueprintResources/StandardMacros.IsValid` _returnvalue
    (:`Is Valid`
      (`EnhancedInputSubsystemInterface.AddMappingContext` _returnvalue "/Game/01-Blueprints/Inputs/IMC_Pirate.IMC_Pirate" 0 (struct))
      (set `self.DefaultRespawnTransform` (`self.GetTransform`))
      (bind _returnvalue_2 (`|CreateWidget` "/Game/01-Blueprints/Widgets/WBP_HUD.WBP_HUD_C"))
      (bind _output_get (set `self.HUDReference` _returnvalue_2))
      (`UserWidget.AddToViewport` _output_get 0))))

(event `EnhancedInput|/Game/01-Blueprints/Inputs/Actions/IA_Pirate_Move`
  (params (ActionValue :type "Vector2D Structure") (ElapsedSeconds :type "Float (double-precision)") (TriggeredSeconds :type "Float (double-precision)") (InputAction :type "InputAction Object Reference" :default "/Game/01-Blueprints/Inputs/Actions/IA_Pirate_Move.IA_Pirate_Move"))
  (bind (_returnvalue_roll _returnvalue_pitch _returnvalue_yaw) (`KismetMathLibrary.BreakRotator` (`self.GetControlRotation`)))
  (bind (_returnvalue_roll_2 _returnvalue_pitch_2 _returnvalue_yaw_2) (`KismetMathLibrary.BreakRotator` (`self.GetControlRotation`)))
  (:`Triggered`
    (`self.AddMovementInput` (`KismetMathLibrary.GetRightVector` (`KismetMathLibrary.MakeRotator` 0.0 0.0 _returnvalue_yaw)) ActionValue_X)
    (`self.AddMovementInput` (`KismetMathLibrary.GetForwardVector` (`KismetMathLibrary.MakeRotator` 0.0 0.0 _returnvalue_yaw_2)) ActionValue_Y)))

(event `EnhancedInput|/Game/01-Blueprints/Inputs/Actions/IA_Pirate_Look`
  (params (ActionValue :type "Vector2D Structure") (ElapsedSeconds :type "Float (double-precision)") (TriggeredSeconds :type "Float (double-precision)") (InputAction :type "InputAction Object Reference" :default "/Game/01-Blueprints/Inputs/Actions/IA_Pirate_Look.IA_Pirate_Look"))
  (:`Triggered`
    (`self.AddControllerYawInput` ActionValue_X)
    (`self.AddControllerPitchInput` ActionValue_Y)))

(event `EnhancedInput|/Game/01-Blueprints/Inputs/Actions/IA_Pirate_Jump`
  (params (ActionValue :type Boolean) (ElapsedSeconds :type "Float (double-precision)") (TriggeredSeconds :type "Float (double-precision)") (InputAction :type "InputAction Object Reference" :default "/Game/01-Blueprints/Inputs/Actions/IA_Pirate_Jump.IA_Pirate_Jump"))
  (:`Started`
    (`self.Jump`))
  (:`Completed`
    (`self.StopJumping`)))

(event `PlayerDeath`
  (`self.K2_SetActorTransform` (`self.DefaultRespawnTransform`) false true))

(event `Checkpoint`
  (params (CheckpointTransform :type "Transform Structure"))
  (set `self.DefaultRespawnTransform` CheckpointTransform))

(event `AddCoin`
  (params (CoinsToAdd :type Integer))
  (bind _output_get (set `self.TotalCoin` (+ (`self.TotalCoin`) CoinsToAdd)))
  (`/Game/01-Blueprints/Widgets/WBP_HUD.UpdateScore` (`self.HUDReference`) _output_get))

(fn `UserConstructionScript`)